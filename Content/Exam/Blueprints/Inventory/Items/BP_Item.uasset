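; BP_Item is an inventory item actor that the top-down character picks up by touching it.
; An overlap on its static mesh casts to BP_TopDownCharacter and passes the item to that character's inventory component through PickItem.
; The item counts as equipment when its EquipmentComponent class is valid, and GetItemType derives one of two enum types from that check.
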(event OnComponentBeginOverlap(StaticMesh)
  (params (OverlappedComponent :type Primitive%20Component%20Object%20Reference) (OtherActor :type Actor%20Object%20Reference) (OtherComp :type Primitive%20Component%20Object%20Reference) (OtherBodyIndex :type Integer) (bFromSweep :type Boolean) (SweepResult :type Hit%20Result%20Structure%20%28by%20ref%29))
  (bind _asbp_top_down_character (Utilities|Casting|CastToBP_TopDownCharacter OtherActor))
  (Default|PickItem (Variables|/Game/Exam/Blueprints/BP_TopDownCharacter.BP_TopDownCharacter_C|GetBP_InventoryComponent _asbp_top_down_character) self))

(fn ConstructionScript)

(fn IsEquipment
  (return (Utilities|IsValidClass (Variables|Default|GetEquipmentComponent))))

(fn GetItemType
  (return (select (CallFunction|IsEquipment) "NewEnumerator1" "NewEnumerator0")))