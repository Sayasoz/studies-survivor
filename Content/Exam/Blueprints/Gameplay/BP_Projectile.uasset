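; BP_Projectile is a reusable bullet actor that can be fired and deactivated without being destroyed.
; FireBullet sets the movement velocity and enables query-only sphere collision, while DeactiveBullet zeroes velocity and disables collision.
; Sphere hits apply damage credited to the instigator; overlaps with actors tagged "None" deactivate the bullet and broadcast OnBulletDestroyed.
; BeginPlay caches the player's top-down character, though nothing here uses it.
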(event OnComponentHit(Sphere)
  (params (HitComponent :type Primitive%20Component%20Object%20Reference) (OtherActor :type Actor%20Object%20Reference) (OtherComp :type Primitive%20Component%20Object%20Reference) (NormalImpulse :type Vector :default "0, 0, 0") (Hit :type Hit%20Result%20Structure%20%28by%20ref%29))
  (CallFunction|ApplyDamage OtherActor))

(event OnComponentBeginOverlap(Sphere)
  (params (OverlappedComponent :type Primitive%20Component%20Object%20Reference) (OtherActor :type Actor%20Object%20Reference) (OtherComp :type Primitive%20Component%20Object%20Reference) (OtherBodyIndex :type Integer) (bFromSweep :type Boolean) (SweepResult :type Hit%20Result%20Structure%20%28by%20ref%29))
  (if (Actor|ActorHasTag OtherActor "None")
    (CallFunction|DeactiveBullet)
    (Default|CallOnBulletDestroyed)))

(event Custom|FireBullet
  (params (Velocity :type Vector))
  (Variables|/Script/Engine.MovementComponent|SetVelocity (Variables|Default|GetProjectileMovement) Velocity)
  (Collision|SetCollisionEnabled (Variables|Default|GetSphere) "QueryOnly"))

(event Custom|DeactiveBullet
  (Variables|/Script/Engine.MovementComponent|SetVelocity (Variables|Default|GetProjectileMovement) "0, 0, 0")
  (Collision|SetCollisionEnabled (Variables|Default|GetSphere) "NoCollision"))

(event EventBeginPlay
  (bind _asbp_top_down_character (Utilities|Casting|CastToBP_TopDownCharacter (Game|GetPlayerCharacter 0)))
  (Variables|Default|SetAs%20BP%20Top%20Down%20Character _asbp_top_down_character))

(fn ConstructionScript)

(fn ApplyDamage
  (params (DamagedActor :type Actor%20Object%20Reference))
  (bind _returnvalue (Game|GetInstigator))
  (Game|Damage|ApplyDamage DamagedActor (Variables|Gameplay|GetDamage) (Game|GetInstigatorController _returnvalue) _returnvalue "/Script/Engine.DamageType"))