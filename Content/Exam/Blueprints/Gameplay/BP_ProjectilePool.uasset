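; BP_ProjectilePool is a projectile pool actor that pre-spawns BP_Projectile instances at its owner's location.
; On BeginPlay it spawns a configurable number, disables their sphere collision, attaches them to the owner and binds each OnBulletDestroyed to ReturnToPool.
; ReturnToPool moves the projectile back to the owner's location and calls attach with no parent actor specified.
; The graph stores no projectile list and has no acquire function.
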(event Custom|ReturnToPool
  (params (Projectile :type BP%20Projectile%20Object%20Reference))
  (Transformation|SetActorLocation Projectile (Transformation|GetActorLocation (Components|GetOwner)) false false)
  (Transformation|AttachActorToActor Projectile 0 "None" "KeepWorld" "KeepWorld" "KeepWorld" true))

(event EventBeginPlay
  (for _index (range 0 (Variables|Default|GetAmmountOfProjectile))
    (bind _returnvalue (Game|SpawnActorfromClass "/Game/Exam/Blueprints/Gameplay/BP_Projectile.BP_Projectile_C" (Math|Transform|MakeTransform (Transformation|GetActorLocation (Components|GetOwner)) "0, 0, 0" "1.000000,1.000000,1.000000") "Undefined" "MultiplyWithRoot" 0 0))
    (Collision|SetCollisionEnabled (Variables|/Game/Exam/Blueprints/Gameplay/BP_Projectile.BP_Projectile_C|GetSphere _returnvalue) "NoCollision")
    (Transformation|AttachActorToActor _returnvalue (Components|GetOwner) "None" "KeepRelative" "KeepRelative" "KeepRelative" true)
    (EventDispatchers|BindEventtoOnBulletDestroyed _returnvalue (delegate Custom|ReturnToPool))))

(fn ConstructionScript)